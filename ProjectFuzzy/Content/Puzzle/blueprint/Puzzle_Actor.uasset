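; Base puzzle pawn that a player possesses on interaction to play an unsolved puzzle, then hands control back to the original character.
; Possession swaps Enhanced Input mappings and interaction enables a cursor highlight; the exit action or a delayed win ends the session.
; Winning sets a flag and fires the PuzzleWon dispatcher, while IsPuzzleWon is a stub returning false.
; A helper toggles custom-depth highlighting on meshes.
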(event `Interact with Puzzle`
  (params (`Player Index` :type Integer))
  (if (not (`self.Puzzle Win Condition?`))
    (bind _output_get (set `self.Player Index` `Player Index`))
    (set `self.Possessing Character` (`GameplayStatics.GetPlayerCharacter` _output_get))
    (`Controller.Possess` (`GameplayStatics.GetPlayerController` _output_get) self)
    (set `PostProcessComponent.bEnabled` true (`self.Cursor Highlight`))))

(event `End Puzzle Active`
  (`Controller.Possess` (`self.GetController` self) (`self.Possessing Character`))
  (set `PostProcessComponent.bEnabled` false (`self.Cursor Highlight`)))

(event `Set Highlight on Mesh Component`
  (params (`Mesh to Highlight` :type "MeshComponent Object Reference") (`Highlight Active` :type Boolean))
  (`PrimitiveComponent.SetRenderCustomDepth` `Mesh to Highlight` `Highlight Active`))

(event `Win Condition Achieved`
  (set `self.Puzzle Win Condition?` true)
  (`self.Puzzle Won`)
  (`KismetSystemLibrary.PrintString` "PUZZLE WON!!!")
  (`KismetSystemLibrary.Delay` (`self.Win Exit Delay`))
  (`self.End Puzzle Active`))

(event `self.ReceivePossessed`
  (params (NewController :type "Controller Object Reference"))
  (bind _asplayer_controller (cast `PlayerController` NewController))
  (bind _returnvalue (pcsubsystem `EnhancedInputLocalPlayerSubsystem` _asplayer_controller))
  (`/Engine/EditorBlueprintResources/StandardMacros.IsValid` _returnvalue
    (:`Is Valid`
      (`EnhancedInputSubsystemInterface.ClearAllMappings` _returnvalue)
      (`EnhancedInputSubsystemInterface.AddMappingContext` _returnvalue "/Game/Puzzle/input/IMC_PlayerControls.IMC_PlayerControls" 0 (struct)))))

(event `self.ReceiveUnpossessed`
  (params (OldController :type "Controller Object Reference"))
  (bind _asplayer_controller (cast `PlayerController` OldController))
  (bind _returnvalue (pcsubsystem `EnhancedInputLocalPlayerSubsystem` _asplayer_controller))
  (`/Engine/EditorBlueprintResources/StandardMacros.IsValid` _returnvalue
    (:`Is Valid`
      (`EnhancedInputSubsystemInterface.ClearAllMappings` _returnvalue))))

(event `EnhancedInput|/Game/Puzzle/input/Actions/IA_ExitPuzzle`
  (params (ActionValue :type Boolean) (ElapsedSeconds :type "Float (double-precision)") (TriggeredSeconds :type "Float (double-precision)") (InputAction :type "InputAction Object Reference" :default "/Game/Puzzle/input/Actions/IA_ExitPuzzle.IA_ExitPuzzle"))
  (:`Triggered`
    (`self.End Puzzle Active`)))

(fn `Get Puzzle Win Condition`
  (returns (`Puzzle Win Condition?` :type Boolean))
  (return (`self.Puzzle Win Condition?`)))

(fn `Is Puzzle Won?`
  (returns (`Puzzle Won?` :type Boolean))
  (return false))

(fn `UserConstructionScript`)